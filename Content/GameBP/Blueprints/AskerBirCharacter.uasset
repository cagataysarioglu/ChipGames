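; AskerBirCharacter is an enemy AI character that wanders, chases the player and takes projectile damage.
; Projectile overlaps show a new HitMarker widget and reduce Health, then either destroy it or spawn an impact emitter and send it toward the player.
; PawnSensing starts a chase of TeomanCharacter and sets CanSeePlayer until that move ends.
; A delay on Tick throttles random nearby wandering while CanSeePlayer is false.
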(event OnSeePawn(PawnSensing)
  (params (Pawn :type Pawn%20Object%20Reference))
  (bind _asteoman_character (Utilities|Casting|CastToTeomanCharacter Pawn))
  (Variables|Default|SetCanSeePlayer true)
  (AI|AIMoveTo self "0, 0, 0" _asteoman_character 5.0 false
    (:OnSuccess
      _)
    (:OnFail
      _))
  (Variables|Default|SetCanSeePlayer false))

(event EventBeginPlay)

(event Collision|EventActorBeginOverlap
  (params (OtherActor :type Actor%20Object%20Reference))
  (bind _asprojectile (Utilities|Casting|CastToProjectile OtherActor))
  (bind _returnvalue (UserInterface|CreateWidget "/Game/UI/HitMarker.HitMarker_C"))
  (UserInterface|Viewport|AddtoViewport _returnvalue 0)
  (Variables|Default|SetHealth (- (Variables|Default|GetHealth) 0.2))
  (if (<= (Variables|Default|GetHealth) 0.0)
    (Actor|DestroyActor)
    (else
      (Effects|SpawnEmitteratLocation 0 (Transformation|GetActorLocation _asprojectile))
      (bind _asteoman_character (Utilities|Casting|CastToTeomanCharacter (Game|GetPlayerCharacter 0)))
      (AI|AIMoveTo self "0, 0, 0" _asteoman_character 5.0 false))))

(event EventTick
  (params (DeltaSeconds :type Float%20%28single-precision%29))
  (Utilities|FlowControl|Delay 3.0)
  (if (not (Variables|Default|GetCanSeePlayer))
    (AI|AIMoveTo self (.RandomLocation (AI|Navigation|GetRandomReachablePointinRadius (Transformation|GetActorLocation) 2.5e+02 0 0)) 0 5.0 false)))

(fn ConstructionScript)