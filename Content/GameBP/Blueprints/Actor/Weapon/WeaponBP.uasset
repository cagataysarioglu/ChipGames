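; Pickable weapon actor for TeomanPlayer that handles pickup, automatic fire and reloading.
; Sphere overlap shows a widget and custom-depth highlight, letting the interact input call PickUp.
; A Gate and RetriggerableDelay loop fires camera line traces, applying random damage through the TakeDamage interface and spawning a muzzle ProjectileBP aimed at the impact, plus effects.
; ItemInfo tracks ammo; releasing fire auto-reloads an empty clip, with fixed delays covering reload montages.
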(event OnComponentBeginOverlap(Sphere)
  (params (OverlappedComponent :type Primitive%20Component%20Object%20Reference) (OtherActor :type Actor%20Object%20Reference) (OtherComp :type Primitive%20Component%20Object%20Reference) (OtherBodyIndex :type Integer) (bFromSweep :type Boolean) (SweepResult :type Hit%20Result%20Structure%20%28by%20ref%29))
  (bind _asteoman_player (Utilities|Casting|CastToTeomanPlayer OtherActor))
  (Variables|Default|SetTeomanReference _asteoman_player)
  (CallFunction|VisibilityCustomDepth true true)
  (Variables|Default|SetIsPickable true)
  (Input|EnableInput (Game|GetPlayerController 0))
  (Physics|SetSimulatePhysics (Variables|Default|GetSkeletalMesh) false))

(event OnComponentEndOverlap(Sphere)
  (params (OverlappedComponent :type Primitive%20Component%20Object%20Reference) (OtherActor :type Actor%20Object%20Reference) (OtherComp :type Primitive%20Component%20Object%20Reference) (OtherBodyIndex :type Integer))
  (bind _asteoman_player (Utilities|Casting|CastToTeomanPlayer OtherActor))
  (Variables|Default|SetTeomanReference _asteoman_player)
  (CallFunction|VisibilityCustomDepth false false)
  (Variables|Default|SetIsPickable false))

(event Custom|OffAll
  (CallFunction|VisibilityCustomDepth false false)
  (Components|DestroyComponent (Variables|Default|GetSphere)))

(event Custom|StartFire
  (bind _skeletalmesh (Variables|Default|GetSkeletalMesh))
  (bind _skeletalmesh_2 (Variables|Default|GetSkeletalMesh))
  (bind _teomanreference (Variables|Default|GetTeomanReference))
  (bind _returnvalue (Transformation|GetSocketLocation _skeletalmesh "Muzzle"))
  (bind _followcamera (Variables|/Game/GameBP/Blueprints/TeomanPlayer.TeomanPlayer_C|GetFollowCamera _teomanreference))
  (bind _returnvalue_2 (Transformation|GetWorldLocation _followcamera))
  (Utilities|FlowControl|Sequence
    (:then_0
      (goto _label Open))
    (:then_1
      (Utilities|FlowControl|Gate true :!label _label
        (:Exit
          (Utilities|FlowControl|Sequence
            (:then_0
              (Utilities|FlowControl|RetriggerableDelay 0.1)
              (goto _label))
            (:then_1
              (if (<= (Utilities|Struct|BreakWeaponInfo (Variables|Default|GetItemInfo)) 0)
                ;[1 1 1] Mermi bittiğinde çıkacak olan ses
                (Audio|PlaySound2D 0 1.0 1.0 0.0 0 0)
                (else
                  (bind (_outhit _returnvalue_3) (Collision|LineTraceByChannel _returnvalue_2 (+ _returnvalue_2 (* (Math|Vector|GetForwardVector _followcamera) 1.3e+04)) "TraceTypeQuery1" false 0 "None"))
                  (if _returnvalue_3
                    _
                    (else
                      _))
                  ;[1 1 1] Ateş etme sesi
                  (Audio|PlaySound2D 0 1.0 1.0 0.0 0 0)
                  (Animation|PlayAnimMontage (Variables|Default|GetTeomanReference) (Variables|Default|GetFireAnimation) 1.0 "None")
                  (Utilities|Struct|SetmembersinWeaponInfo (Variables|Default|GetItemInfo) (- (Utilities|Struct|BreakWeaponInfo (Variables|Default|GetItemInfo)) 1))
                  (if (Utilities|DoesObjectImplementInterface (.HitActor (Collision|BreakHitResult _outhit)) "/Game/GameBP/Blueprints/AI/TakeDamage.TakeDamage_C")
                    (Class|TakeDamage|ITakeDamage(Message) (.HitActor (Collision|BreakHitResult _outhit)) (.HitBoneName (Collision|BreakHitResult _outhit)) (Math|Random|RandomFloatinRange 2e+01 35.0)))
                  (Game|SpawnActorfromClass "/Game/GameBP/Blueprints/Actor/Bullet/ProjectileBP.ProjectileBP_C" (Math|Transform|MakeTransform _returnvalue (Math|Rotator|FindLookatRotation _returnvalue (Math|Vector|SelectVector (.ImpactPoint (Collision|BreakHitResult _outhit)) (.TraceEnd (Collision|BreakHitResult _outhit)) _returnvalue_3))) "Undefined" 0 0)
                  (Effects|SpawnEmitterAttached 0 _skeletalmesh_2 "Muzzle" (Transformation|GetSocketLocation _skeletalmesh_2 "Muzzle") "0, 0, 0" (Math|Rotator|GetRotationXVector (Transformation|GetSocketRotation _skeletalmesh_2 "Muzzle")) "KeepWorldPosition")
                  (Effects|SpawnEmitteratLocation 0 (.Location (Collision|BreakHitResult _outhit))))))))))))

(event Custom|StopFire
  (bind _skeletalmesh (Variables|Default|GetSkeletalMesh))
  (bind _skeletalmesh_2 (Variables|Default|GetSkeletalMesh))
  (bind _teomanreference (Variables|Default|GetTeomanReference))
  (bind _returnvalue (Transformation|GetSocketLocation _skeletalmesh "Muzzle"))
  (bind _followcamera (Variables|/Game/GameBP/Blueprints/TeomanPlayer.TeomanPlayer_C|GetFollowCamera _teomanreference))
  (bind _returnvalue_2 (Transformation|GetWorldLocation _followcamera))
  (Utilities|FlowControl|Gate true) ; enters at Close
)

(event Custom|FirePress
  (Variables|Default|SetCanFire true)
  (if (not (Variables|Default|GetIsReloading))
    (CallFunction|StartFire)))

(event Custom|FireRelease
  (Variables|Default|SetCanFire false)
  (CallFunction|StopFire)
  (CallFunction|AutoReload))

(event Custom|Reloading
  (bind _iteminfo (Variables|Default|GetItemInfo))
  (bind (_clipsize _currentammo) (Utilities|Struct|BreakWeaponInfo _iteminfo))
  (if (== (Utilities|Struct|BreakWeaponInfo (Variables|Default|GetItemInfo)) 0)
    ;[1 1 1] Yüklenecek mühimmat bulunmadığında çıkacak olan ses
    (Audio|PlaySound2D 0 1.0 1.0 0.0 0 0)
    (elif (== _clipsize _currentammo)
      ;[1 1 1] Şarjör dolu olduğunda çıkacak olan ses
      (Audio|PlaySound2D 0 1.0 1.0 0.0 0 0)
      (else
        (bind _output_get (Variables|Default|SetIsReloading true))
        (if _output_get
          (CallFunction|WeaponReload)
          (Utilities|FlowControl|Delay 3.3) ; Yükleme animasyon süresi
          (Variables|Default|SetIsReloading false))))))

(event Custom|WeaponReload
  (bind _iteminfo (Variables|Default|GetItemInfo))
  (bind _iteminfo_2 (Variables|Default|GetItemInfo))
  (bind _iteminfo_3 (Variables|Default|GetItemInfo))
  (bind _iteminfo_4 (Variables|Default|GetItemInfo))
  (bind (_clipsize _currentammo) (Utilities|Struct|BreakWeaponInfo _iteminfo_3))
  (bind _maxammo (Utilities|Struct|BreakWeaponInfo _iteminfo_4))
  (bind (_currentammo_2 _maxammo_2) (Utilities|Struct|BreakWeaponInfo _iteminfo))
  (if (not (Variables|Default|GetCanFire))
    ;[1 1 1] Şarjör yükleme sesi
    (Audio|PlaySound2D 0 1.0 1.0 0.0 0 0)
    (Animation|PlayAnimMontage (Variables|Default|GetTeomanReference) "/Game/Models/Animations/Teoman/TufekYuklemeMontage.TufekYuklemeMontage" 1.0 "None")
    (if (> (Utilities|Struct|BreakWeaponInfo (Variables|Default|GetItemInfo)) 0)
      (Variables|Default|SetNeededAmmo (- _clipsize _currentammo))
      (if (<= _maxammo (Variables|Default|GetNeededAmmo))
        (Utilities|Struct|SetmembersinWeaponInfo _iteminfo_2 (+ _currentammo_2 _maxammo_2))
        (Utilities|Struct|SetmembersinWeaponInfo _iteminfo_2)
        (else
          (Utilities|Struct|SetmembersinWeaponInfo _iteminfo_2 (- _maxammo (Variables|Default|GetNeededAmmo)))
          (Utilities|Struct|SetmembersinWeaponInfo _iteminfo_2 (Utilities|Struct|BreakWeaponInfo (Variables|Default|GetItemInfo))))))))

(event Custom|AutoReload
  (if (== (Utilities|Struct|BreakWeaponInfo (Variables|Default|GetItemInfo)) 0)
    (if (== (Utilities|Struct|BreakWeaponInfo (Variables|Default|GetItemInfo)) 0)
      ;[1 1 1] Mühimmat bulunması gerektiğinde çıkacak olan ses
      (Audio|PlaySound2D 0 1.0 1.0 0.0 0 0)
      (else
        (Variables|Default|SetIsReloading true)
        (CallFunction|Reloading)
        (Utilities|FlowControl|Delay 3.3) ; Yükleme animasyon süresi
        (Variables|Default|SetIsReloading false)))))

(event Custom|DestroySphere
  (Components|DestroyComponent (Variables|Default|GetSphere)))

(event EventBeginPlay
  (Rendering|SetVisibility (Variables|Default|GetWidget) false false))

(event Input|ActionEvents|InputActionObjectInteraction
  (params (Key :type Key%20Structure :default "None"))
  (:Pressed
    (if (Variables|Default|GetIsPickable)
      (Default|PickUp (Variables|Default|GetTeomanReference) self))))

(fn ConstructionScript
  (Variables|Default|SetItemInfo (Utilities|Struct|MakeWeaponInfo (.weapontype (Variables|Default|GetItemInfo)) (Utilities|GetClass self) (.clipsize (Variables|Default|GetItemInfo)) (.currentammo (Variables|Default|GetItemInfo)) (.maxammo (Variables|Default|GetItemInfo)) (.damage (Variables|Default|GetItemInfo)) (.weaponimage (Variables|Default|GetItemInfo)) (.equipsocket (Variables|Default|GetItemInfo)) (.unequipsocket (Variables|Default|GetItemInfo)) (.name (Variables|Default|GetItemInfo)))))

(fn VisibilityCustomDepth
  (params (bNewVisibility :type Boolean) (bValue :type Boolean))
  (Rendering|SetVisibility (Variables|Default|GetWidget) bNewVisibility false)
  (Rendering|SetRenderCustomDepth (Variables|Default|GetSkeletalMesh) bValue))