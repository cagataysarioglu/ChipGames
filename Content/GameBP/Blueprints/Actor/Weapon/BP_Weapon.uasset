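; BP_Weapon is an interactable weapon actor that players can pick up and that can be dropped.
; SetWeaponState switches between Dropped, with mesh physics and an overlap sphere, and Equipped, with physics and collision off and the mesh's relative transform reset.
; It starts Dropped, and interaction passes it to the player's PickUpWeapon before setting Equipped.
; Interaction getters supply a Turkish prompt and the skeletal mesh as its attach point.
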(event EventBeginPlay
  (Private|SetWeaponState "NewEnumerator0"))

(event EventOnInteracted
  (params (Player :type Teoman%20Character%20Object%20Reference))
  (Default|PickUpWeapon Player self)
  (Private|SetWeaponState "NewEnumerator1"))

(fn ConstructionScript
  (|CallParentFunction))

(fn GetInteractionText
  (return "ile kuşan"))

(fn GetInteractionTextAttach
  (return (Variables|Default|GetSkeletalMesh)))

(fn SetWeaponState
  (params (WeaponStateInput :type WeaponState%20Enum :default "NewEnumerator0"))
  (bind _skeletalmesh (Variables|Default|GetSkeletalMesh))
  (bind _skeletalmesh_2 (Variables|Default|GetSkeletalMesh))
  (bind _output_get (Variables|Private|SetWeapon%20State WeaponStateInput))
  (switch Utilities|FlowControl|Switch|SwitchonWeaponState _output_get
    (:NewEnumerator0
      (Collision|SetCollisionProfileName (Variables|Default|GetSphere) "OverlapAllDynamic" true :!class /Script/Engine.PrimitiveComponent)
      (Physics|SetSimulatePhysics _skeletalmesh_2 true)
      (Collision|SetCollisionProfileName _skeletalmesh_2 "DroppedWeapon" true :!class /Script/Engine.PrimitiveComponent))
    (:NewEnumerator1
      (Collision|SetCollisionProfileName (Variables|Default|GetSphere) "NoCollision" true :!class /Script/Engine.PrimitiveComponent)
      (Physics|SetSimulatePhysics _skeletalmesh false)
      (Collision|SetCollisionProfileName _skeletalmesh "NoCollision" true :!class /Script/Engine.PrimitiveComponent)
      (Transformation|ResetRelativeTransform (Variables|Default|GetSkeletalMesh)))))

(fn Drop
  (Private|SetWeaponState "NewEnumerator0"))