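; ItemBP is a pickup actor that serves as a health pack, key or quest item, chosen by its Item value.
; Sphere overlap with TeomanPlayer toggles custom-depth highlighting, the prompt widget and CanPick, enabling input on entry.
; Pressing ObjectInteraction while CanPick is set increments the matching player counter.
; Health packs and quest items then play a sound and destroy themselves, while keys do neither because those nodes are disconnected.
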(event OnComponentBeginOverlap(Sphere)
  (params (OverlappedComponent :type Primitive%20Component%20Object%20Reference) (OtherActor :type Actor%20Object%20Reference) (OtherComp :type Primitive%20Component%20Object%20Reference) (OtherBodyIndex :type Integer) (bFromSweep :type Boolean) (SweepResult :type Hit%20Result%20Structure%20%28by%20ref%29))
  (Utilities|Casting|CastToTeomanPlayer OtherActor)
  (Rendering|SetRenderCustomDepth (Variables|Default|GetStaticMesh) true)
  (Rendering|SetVisibility (Variables|Default|GetWidget) true false)
  (Variables|Default|SetCanPick true)
  (Input|EnableInput (Game|GetPlayerController 0)))

(event OnComponentEndOverlap(Sphere)
  (params (OverlappedComponent :type Primitive%20Component%20Object%20Reference) (OtherActor :type Actor%20Object%20Reference) (OtherComp :type Primitive%20Component%20Object%20Reference) (OtherBodyIndex :type Integer))
  (Utilities|Casting|CastToTeomanPlayer OtherActor)
  (Rendering|SetRenderCustomDepth (Variables|Default|GetStaticMesh) false)
  (Rendering|SetVisibility (Variables|Default|GetWidget) false false)
  (Variables|Default|SetCanPick false))

(event Input|ActionEvents|InputActionObjectInteraction
  (params (Key :type Key%20Structure :default "None"))
  (:Pressed
    (if (Variables|Default|GetCanPick)
      (switch Utilities|FlowControl|Switch|SwitchonItemEnumerator (Variables|Default|GetItem)
        (:NewEnumerator1
          (bind _asteoman_player (Utilities|Casting|CastToTeomanPlayer (Game|GetPlayerCharacter 0)))
          (bind _result (Math|Integer|IncrementInt (Variables|/Script/SavgaProject.PlayerCharacterBase|GetHealthPack _asteoman_player))
            (:%20%20
              (Variables|/Script/SavgaProject.PlayerCharacterBase|SetHealthPack _asteoman_player _result)
              (Audio|PlaySound2D 0 1.0 1.0 0.0 0 0)
              (Actor|DestroyActor))))
        (:NewEnumerator2
          (bind _asteoman_player_2 (Utilities|Casting|CastToTeomanPlayer (Game|GetPlayerCharacter 0)))
          (bind _result_2 (Math|Integer|IncrementInt (Variables|/Script/SavgaProject.PlayerCharacterBase|GetDoorKey _asteoman_player_2))
            (:%20%20
              (Variables|/Script/SavgaProject.PlayerCharacterBase|SetDoorKey _asteoman_player_2 _result_2))))
        (:NewEnumerator3
          (bind _asteoman_player_3 (Utilities|Casting|CastToTeomanPlayer (Game|GetPlayerCharacter 0)))
          (bind _result_3 (Math|Integer|IncrementInt (Variables|/Script/SavgaProject.PlayerCharacterBase|GetQuestItem _asteoman_player_3))
            (:%20%20
              (Variables|/Script/SavgaProject.PlayerCharacterBase|SetQuestItem _asteoman_player_3 _result_3)
              (Audio|PlaySound2D 0 1.0 1.0 0.0 0 0)
              (Actor|DestroyActor))))))))

(fn ConstructionScript)