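; DoorBP is a key-locked door that the TeomanPlayer opens and closes with the ObjectInteraction input.
; Box overlap shows an outline and prompt widget, checks the player's DoorKey count, and with a key enables input and marks the door openable.
; Separate timelines swing the actor's yaw from its starting angle, with sounds for opening, closing and locked attempts.
; Leaving the box clears openability but never disables input.
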(event OnComponentBeginOverlap(Box)
  (params (OverlappedComponent :type Primitive%20Component%20Object%20Reference) (OtherActor :type Actor%20Object%20Reference) (OtherComp :type Primitive%20Component%20Object%20Reference) (OtherBodyIndex :type Integer) (bFromSweep :type Boolean) (SweepResult :type Hit%20Result%20Structure%20%28by%20ref%29))
  (bind _asteoman_player (Utilities|Casting|CastToTeomanPlayer OtherActor))
  (Variables|Default|SetTeomanReference _asteoman_player)
  (Rendering|SetRenderCustomDepth (Variables|Default|GetStaticMesh) true)
  (Rendering|SetVisibility (Variables|Default|GetWidget) true false)
  (if (>= (Variables|/Game/GameBP/Blueprints/TeomanPlayer.TeomanPlayer_C|GetDoorKey (Variables|Default|GetTeomanReference)) 1)
    (bind _asdoor_locked_interaction_widget (Utilities|Casting|CastToDoorLockedInteractionWidget (UserInterface|GetUserWidgetObject (Variables|Default|GetWidget))))
    (Variables|/Game/UI/DoorLockedInteractionWidget.DoorLockedInteractionWidget_C|SetKeyText _asdoor_locked_interaction_widget "Aç-kapat")
    (Input|EnableInput (Game|GetPlayerController 0))
    (Variables|Default|SetIsOpenable true)
    (else
      (bind _asdoor_locked_interaction_widget_2 (Utilities|Casting|CastToDoorLockedInteractionWidget (UserInterface|GetUserWidgetObject (Variables|Default|GetWidget))))
      (Variables|/Game/UI/DoorLockedInteractionWidget.DoorLockedInteractionWidget_C|SetKeyText _asdoor_locked_interaction_widget_2 "Anahtarı bul")
      (Variables|Default|SetIsOpenable false))))

(event OnComponentEndOverlap(Box)
  (params (OverlappedComponent :type Primitive%20Component%20Object%20Reference) (OtherActor :type Actor%20Object%20Reference) (OtherComp :type Primitive%20Component%20Object%20Reference) (OtherBodyIndex :type Integer))
  (bind _asteoman_player (Utilities|Casting|CastToTeomanPlayer OtherActor))
  (Variables|Default|SetTeomanReference _asteoman_player)
  (Rendering|SetRenderCustomDepth (Variables|Default|GetStaticMesh) false)
  (Rendering|SetVisibility (Variables|Default|GetWidget) false false)
  (Variables|Default|SetIsOpenable false))

(event EventBeginPlay
  (Variables|Default|SetCurrentAngle (Transformation|GetActorRotation)))

(event Input|ActionEvents|InputActionObjectInteraction
  (params (Key :type Key%20Structure :default "None"))
  (bind _staticmesh (Variables|Default|GetStaticMesh))
  (bind _returnvalue (Transformation|GetWorldLocation _staticmesh))
  (:Pressed
    (if (Variables|Default|GetIsOpenable)
      (if (Variables|Default|GetIsDoorOpen)
        ;[1 1 1] Kapı kapanma sesi
        (Audio|PlaySoundatLocation 0 _returnvalue "0, 0, 0" 1.0 1.0 0.0 0 0 0)
        (bind _close (Timeline|CloseDoor ReverseFromEnd)
          (:Update
            (Transformation|SetActorRelativeRotation (Math|Rotator|MakeRotator 0.0 0.0 (+ (.yaw (Variables|Default|GetCurrentAngle)) _close)))
            (Variables|Default|SetIsDoorOpen false)))
        (else
          ;[1 1 1] Kapı açılma sesi
          (Audio|PlaySoundatLocation 0 _returnvalue "0, 0, 0" 1.0 1.0 0.0 0 0 0)
          (bind _open (Timeline|OpenDoor PlayFromStart)
            (:Update
              (Transformation|SetActorRelativeRotation (Math|Rotator|MakeRotator 0.0 0.0 (+ (.yaw (Variables|Default|GetCurrentAngle)) _open)))
              (Variables|Default|SetIsDoorOpen true)))))
      (else
        ;[1 1 1] Kilitli kapı sesi
        (Audio|PlaySoundatLocation 0 _returnvalue "0, 0, 0" 1.0 1.0 0.0 0 0 0)))))

(fn ConstructionScript)