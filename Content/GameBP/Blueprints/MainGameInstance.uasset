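; Game instance that handles save slots, menu display and level unlocking.
; LoadGame loads or creates a MainSaveGame, starting a looping AutoSave timer only when a save already exists.
; SavePlayerData and LoadPlayerData copy TeomanPlayer state to and from that object, with helpers to read or delete slots.
; Show events spawn menu widgets with the cursor visible, and UnlockLevel increments a counter that sets per-level flags, which are not saved here.
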(event Custom|ShowMainMenu
  (bind _returnvalue (Game|GetPlayerController 0))
  (bind _returnvalue_2 (UserInterface|CreateWidget "/Game/UI/Menu/MainMenuWBP.MainMenuWBP_C" _returnvalue))
  (UserInterface|Viewport|AddtoViewport _returnvalue_2 0)
  (Variables|/Script/Engine.PlayerController|SetbShowMouseCursor _returnvalue true)
  (Utilities|FlowControl|DoOnce false
    (:Completed
      (Audio|PlaySound2D "/Game/Sounds/Closing_In.Closing_In" 1.0 1.0 0.0 0 0))))

(event Custom|ShowMapMenu
  (bind _returnvalue (Game|GetPlayerController 0))
  (bind _returnvalue_2 (UserInterface|CreateWidget "/Game/UI/Menu/MapMenuWBP.MapMenuWBP_C" _returnvalue))
  (UserInterface|Viewport|AddtoViewport _returnvalue_2 0)
  (Variables|/Script/Engine.PlayerController|SetbShowMouseCursor _returnvalue true))

(event Custom|ShowSettingsMenu
  (bind _returnvalue (Game|GetPlayerController 0))
  (bind _returnvalue_2 (UserInterface|CreateWidget "/Game/UI/Menu/SettingsMenuWBP.SettingsMenuWBP_C" _returnvalue))
  (UserInterface|Viewport|AddtoViewport _returnvalue_2 0)
  (Variables|/Script/Engine.PlayerController|SetbShowMouseCursor _returnvalue true))

(event Custom|ShowQuitMenu
  (bind _returnvalue (Game|GetPlayerController 0))
  (bind _returnvalue_2 (UserInterface|CreateWidget "/Game/UI/Menu/QuitMenuWBP.QuitMenuWBP_C" _returnvalue))
  (UserInterface|Viewport|AddtoViewport _returnvalue_2 0)
  (Variables|/Script/Engine.PlayerController|SetbShowMouseCursor _returnvalue true))

(event Custom|ShowCredits
  (bind _returnvalue (Game|GetPlayerController 0))
  (bind _returnvalue_2 (UserInterface|CreateWidget "/Game/UI/Menu/CreditsMenuWBP.CreditsMenuWBP_C" _returnvalue))
  (UserInterface|Viewport|AddtoViewport _returnvalue_2 0)
  (Variables|/Script/Engine.PlayerController|SetbShowMouseCursor _returnvalue true))

(event Custom|ShowLoadMenu
  (bind _returnvalue (Game|GetPlayerController 0))
  (bind _returnvalue_2 (UserInterface|CreateWidget "/Game/UI/Menu/LoadMenuWBP.LoadMenuWBP_C" _returnvalue))
  (UserInterface|Viewport|AddtoViewport _returnvalue_2 0)
  (Variables|/Script/Engine.PlayerController|SetbShowMouseCursor _returnvalue true))

(event Custom|LoadGame
  (params (SaveSlotName :type String))
  (bind _output_get (Variables|Default|SetSaveSlotName SaveSlotName))
  (bind _returnvalue (SaveGame|DoesSaveGameExist _output_get))
  (if _returnvalue
    (bind _returnvalue_2 (SaveGame|LoadGamefromSlot (Variables|Default|GetSaveSlotName)))
    (bind _asmain_save_game (Utilities|Casting|CastToMainSaveGame _returnvalue_2))
    (Variables|Default|SetSaveGameData _asmain_save_game)
    (Utilities|Time|SetTimerbyFunctionName self "AutoSave" 4e+04 true)
    (else
      (bind _returnvalue_3 (SaveGame|CreateSaveGameObject "/Game/GameBP/Blueprints/MainSaveGame.MainSaveGame_C"))
      (Variables|Default|SetSaveGameData _returnvalue_3))))

(fn UnlockLevel
  (bind _result (Math|Integer|IncrementInt (Variables|Default|GetLevelUnlock))
    (:%20%20
      (Variables|Default|SetLevelUnlock _result)
      (if (== (Variables|Default|GetLevelUnlock) 1)
        (Variables|Default|SetLevel_2 true)
        (elif (== (Variables|Default|GetLevelUnlock) 2)
          (Variables|Default|SetLevel_3 true)
          (elif (== (Variables|Default|GetLevelUnlock) 3)
            (Variables|Default|SetLevel_4 true)
            (elif (== (Variables|Default|GetLevelUnlock) 4)
              (Variables|Default|SetLevel_5 true)
              (elif (== (Variables|Default|GetLevelUnlock) 5)
                (Variables|Default|SetLevel_6 true)
                (elif (== (Variables|Default|GetLevelUnlock) 6)
                  (Variables|Default|SetLevel_7 true))))))))))

(fn SavePlayerData
  (bind _asteoman_player (Utilities|Casting|CastToTeomanPlayer (Game|GetPlayerCharacter 0)))
  (bind _output_get (LocalVariables|SetPlayerReference _asteoman_player))
  (Variables|/Game/GameBP/Blueprints/MainSaveGame.MainSaveGame_C|SetPlayerData (Variables|Default|GetSaveGameData) (Utilities|Struct|MakePlayerSaveData (Variables|/Game/GameBP/Blueprints/TeomanPlayer.TeomanPlayer_C|GetLevelName _output_get) (Transformation|GetActorLocation _output_get) (Variables|/Game/GameBP/Blueprints/TeomanPlayer.TeomanPlayer_C|GetObjectiveText _output_get) (Variables|/Game/GameBP/Blueprints/TeomanPlayer.TeomanPlayer_C|GetCurrentHealth _output_get) (Variables|/Game/GameBP/Blueprints/TeomanPlayer.TeomanPlayer_C|GetHealthKit _output_get) (Variables|/Game/GameBP/Blueprints/Actor/Weapon/WeaponBP.WeaponBP_C|GetItemInfo (Variables|/Game/GameBP/Blueprints/TeomanPlayer.TeomanPlayer_C|GetPrimaryRifle _output_get)) (Variables|/Game/GameBP/Blueprints/TeomanPlayer.TeomanPlayer_C|GetDoorKey _output_get) (Variables|/Game/GameBP/Blueprints/TeomanPlayer.TeomanPlayer_C|GetQuestItem _output_get)))
  (SaveGame|SaveGametoSlot (Variables|Default|GetSaveGameData) (Variables|Default|GetSaveSlotName)))

(fn LoadPlayerData
  (bind _asteoman_player (Utilities|Casting|CastToTeomanPlayer (Game|GetPlayerCharacter 0)))
  (bind _output_get (LocalVariables|SetPlayerReference _asteoman_player))
  (bind _savegamedata (Variables|Default|GetSaveGameData)
    (:then
      (Variables|/Game/GameBP/Blueprints/TeomanPlayer.TeomanPlayer_C|SetLevelName _output_get (.level (Variables|/Game/GameBP/Blueprints/MainSaveGame.MainSaveGame_C|GetPlayerData _savegamedata)))
      (Transformation|SetActorLocation _output_get (.location (Variables|/Game/GameBP/Blueprints/MainSaveGame.MainSaveGame_C|GetPlayerData _savegamedata)) false false)
      (Variables|/Game/GameBP/Blueprints/TeomanPlayer.TeomanPlayer_C|SetObjectiveText _output_get (.quest (Variables|/Game/GameBP/Blueprints/MainSaveGame.MainSaveGame_C|GetPlayerData _savegamedata)))
      (Variables|/Game/GameBP/Blueprints/TeomanPlayer.TeomanPlayer_C|SetCurrentHealth _output_get (.health (Variables|/Game/GameBP/Blueprints/MainSaveGame.MainSaveGame_C|GetPlayerData _savegamedata)))
      (Variables|/Game/GameBP/Blueprints/TeomanPlayer.TeomanPlayer_C|SetHealthKit _output_get (.healthpack (Variables|/Game/GameBP/Blueprints/MainSaveGame.MainSaveGame_C|GetPlayerData _savegamedata)))
      (Variables|/Game/GameBP/Blueprints/Actor/Weapon/WeaponBP.WeaponBP_C|SetItemInfo (Variables|/Game/GameBP/Blueprints/TeomanPlayer.TeomanPlayer_C|GetPrimaryRifle _output_get) (.weapon (Variables|/Game/GameBP/Blueprints/MainSaveGame.MainSaveGame_C|GetPlayerData _savegamedata)))
      (Variables|/Game/GameBP/Blueprints/TeomanPlayer.TeomanPlayer_C|SetDoorKey _output_get (.key (Variables|/Game/GameBP/Blueprints/MainSaveGame.MainSaveGame_C|GetPlayerData _savegamedata)))
      (Variables|/Game/GameBP/Blueprints/TeomanPlayer.TeomanPlayer_C|SetQuestItem _output_get (.questitem (Variables|/Game/GameBP/Blueprints/MainSaveGame.MainSaveGame_C|GetPlayerData _savegamedata))))
    (:else)))

(fn ClearSavedData
  (SaveGame|DeleteGameinSlot (Variables|Default|GetSaveSlotName)))

(fn AutoSave
  (CallFunction|SavePlayerData))

(fn RetrieveSaveData
  (params (LOCAL_SaveSlotName :type String))
  (bind _returnvalue (SaveGame|DoesSaveGameExist LOCAL_SaveSlotName))
  (if _returnvalue
    (bind _returnvalue_2 (SaveGame|LoadGamefromSlot LOCAL_SaveSlotName))
    (bind _asmain_save_game (Utilities|Casting|CastToMainSaveGame _returnvalue_2))
    (return (Variables|/Game/GameBP/Blueprints/MainSaveGame.MainSaveGame_C|GetPlayerData _asmain_save_game))))