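; Game mode that manages save data, keeping a separate LevelSaveGame slot per level, named after the current level.
; On BeginPlay it loads or creates the level save object, then calls LoadWeapons on it.
; SaveLevelData writes that object back to the level's slot.
; InitPlayerSaveData similarly loads or creates a PlayerSaveGame from the "PlayerData" slot, but nothing in this graph calls it.
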(event EventBeginPlay
  (CallFunction|InitLevelSaveData)
  (Default|LoadWeapons (Variables|Default|GetLevelSaveObject)))

(fn ConstructionScript)

(fn InitLevelSaveData
  (bind _returnvalue (Game|GetCurrentLevelName true))
  (bind _returnvalue_2 (SaveGame|DoesSaveGameExist _returnvalue))
  (if _returnvalue_2
    (bind _returnvalue_3 (Game|GetCurrentLevelName true))
    (bind _returnvalue_4 (SaveGame|LoadGamefromSlot _returnvalue_3))
    (bind _aslevel_save_game (Utilities|Casting|CastToLevelSaveGame _returnvalue_4))
    (Variables|Default|SetLevelSaveObject _aslevel_save_game)
    (else
      (bind _returnvalue_5 (SaveGame|CreateSaveGameObject "/Game/GameBP/Blueprints/LevelSaveGame.LevelSaveGame_C"))
      (Variables|Default|SetLevelSaveObject _returnvalue_5))))

(fn InitPlayerSaveData
  (bind _returnvalue (SaveGame|DoesSaveGameExist "PlayerData"))
  (if _returnvalue
    (bind _returnvalue_2 (SaveGame|LoadGamefromSlot "PlayerData"))
    (bind _asplayer_save_game (Utilities|Casting|CastToPlayerSaveGame _returnvalue_2))
    (Variables|Default|SetPlayerSaveObject _asplayer_save_game)
    (else
      (bind _returnvalue_3 (SaveGame|CreateSaveGameObject "/Game/GameBP/Blueprints/PlayerSaveGame.PlayerSaveGame_C"))
      (Variables|Default|SetPlayerSaveObject _returnvalue_3))))

(fn SaveLevelData
  (bind _returnvalue (Game|GetCurrentLevelName true))
  (SaveGame|SaveGametoSlot (Variables|Default|GetLevelSaveObject) _returnvalue))