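; AI controller for the AskerYZ_BP soldier that patrols waypoints back and forth, then hunts and shoots the player.
; A looping timer polls the pawn's EnemyFound flag and both death states to trigger hunting, resume patrol or stop.
; Hunting moves toward the player, toggling fire and acceptance radius from the pawn's Active flag.
; Firing loops through a Gate with random delays, applying line-trace damage via interface and spawning a projectile toward the hit.
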(event Custom|Patrolling
  (if (not (Variables|Default|GetFoundEnemy))
    (if (Variables|Default|GetWalkBack)
      (Math|Integer|DecrementInt (Variables|Default|GetCurrentWayPoint)
        (:%20%20
          (AI|AIMoveTo 0 "0, 0, 0" (Utilities|Array|Get(acopy) (Variables|Default|GetWayPoints) (Variables|Default|GetCurrentWayPoint)) 5.0 false
            (:OnSuccess
              (if (<= (Variables|Default|GetCurrentWayPoint) 0)
                (Variables|Default|SetWalkBack false))))))
      (else
        (Math|Integer|IncrementInt (Variables|Default|GetCurrentWayPoint)
          (:%20%20
            (AI|AIMoveTo 0 "0, 0, 0" (Utilities|Array|Get(acopy) (Variables|Default|GetWayPoints) (Variables|Default|GetCurrentWayPoint)) 5.0 false
              (:OnSuccess
                (if (>= (Variables|Default|GetCurrentWayPoint) (- (Utilities|Array|Length (Variables|Default|GetWayPoints)) 1))
                  (Variables|Default|SetWalkBack true))))))))
    (Utilities|FlowControl|Delay 4.0)
    (CallFunction|Patrolling)))

(event Custom|OnHunt
  (AI|AIMoveTo 0 "0, 0, 0" (Game|GetPlayerCharacter 0) (Variables|Default|GetRadius) false
    (:OnSuccess
      _)
    (:OnFail
      _))
  (if (Variables|/Game/GameBP/Blueprints/AI/AskerYZ_BP.AskerYZ_BP_C|GetActive (Variables|Default|GetAIBaseReference))
    (CallFunction|Fire)
    (Variables|Default|SetRadius 1.7e+03)
    (else
      (CallFunction|StopFire)
      (Variables|Default|SetRadius 1e+02))))

(event Custom|CheckEnemy
  (bind _aibasereference (Variables|Default|GetAIBaseReference))
  (if (Variables|/Game/GameBP/Blueprints/TeomanPlayer.TeomanPlayer_C|GetIsDead (.AsTeoman%20Player (Utilities|Casting|CastToTeomanPlayer (Game|GetPlayerCharacter 0))))
    (Variables|Default|SetFoundEnemy false)
    (Utilities|FlowControl|DoOnce false
      (:Completed
        (Default|EnableCombat (Variables|Default|GetAIBaseReference))
        (Utilities|FlowControl|Delay 2.0)
        (CallFunction|Patrolling)))
    (elif (Variables|/Game/GameBP/Blueprints/AI/AskerYZ_BP.AskerYZ_BP_C|GetIsDead _aibasereference)
      (Utilities|Time|ClearandInvalidateTimerbyHandle (Variables|Default|GetCleanTimer))
      (AI|Navigation|StopMovement)
      (else
        (bind _output_get (Variables|Default|SetFoundEnemy (Variables|/Game/GameBP/Blueprints/AI/AskerYZ_BP.AskerYZ_BP_C|GetEnemyFound _aibasereference)))
        (if _output_get
          (Utilities|FlowControl|Sequence
            (:then_0
              (Default|ScanEnemy (Variables|Default|GetAIBaseReference))
              (CallFunction|OnHunt))
            (:then_1
              (Utilities|FlowControl|DoOnce false
                (:Completed
                  (Default|EnableCombat (Variables|Default|GetAIBaseReference)))))))))))

(event Custom|Fire
  (bind _aibasereference (Variables|Default|GetAIBaseReference))
  (bind _aibasereference_2 (Variables|Default|GetAIBaseReference))
  (bind _weapon (Variables|/Game/GameBP/Blueprints/AI/AskerYZ_BP.AskerYZ_BP_C|GetWeapon _aibasereference))
  (bind _weapon_2 (Variables|/Game/GameBP/Blueprints/AI/AskerYZ_BP.AskerYZ_BP_C|GetWeapon _aibasereference_2))
  (bind _skeletalmesh (Variables|/Game/GameBP/Blueprints/Actor/Weapon/WeaponBP.WeaponBP_C|GetSkeletalMesh _weapon))
  (bind _skeletalmesh_2 (Variables|/Game/GameBP/Blueprints/Actor/Weapon/WeaponBP.WeaponBP_C|GetSkeletalMesh _weapon_2))
  (bind _returnvalue (Transformation|GetSocketLocation _skeletalmesh "Muzzle"))
  (bind _returnvalue_2 (Transformation|GetSocketLocation _skeletalmesh_2 "Muzzle"))
  (Utilities|FlowControl|Sequence
    (:then_0
      (goto _label Open))
    (:then_1
      (Utilities|FlowControl|Gate true :!label _label
        (:Exit
          (Utilities|FlowControl|Sequence
            (:then_0
              (Utilities|FlowControl|RetriggerableDelay (Math|Random|RandomFloatinRange (Math|Random|RandomFloatinRange 0.2 0.3) (Math|Random|RandomFloatinRange 0.7 1.0)))
              (if (not (Variables|/Game/GameBP/Blueprints/AI/AskerYZ_BP.AskerYZ_BP_C|GetIsDead (Variables|Default|GetAIBaseReference)))
                (goto _label)))
            (:then_1
              (bind (_outhit _returnvalue_3) (Collision|LineTraceByChannel _returnvalue_2 (+ _returnvalue_2 (* (Math|Vector|GetForwardVector _skeletalmesh_2) 3e+03)) "TraceTypeQuery1" true 0 "None"))
              (if _returnvalue_3
                _
                (else
                  _))
              ;[1 1 1] Ateş etme sesi
              (Audio|PlaySound2D 0 1.0 1.0 0.0 0 0)
              (if (Utilities|DoesObjectImplementInterface (.HitActor (Collision|BreakHitResult _outhit)) "/Game/GameBP/Blueprints/AI/TakeDamage.TakeDamage_C")
                (Class|TakeDamage|ITakeDamage(Message) (.HitActor (Collision|BreakHitResult _outhit)) (.HitBoneName (Collision|BreakHitResult _outhit)) (Math|Random|RandomFloatinRange 2e+01 35.0)))
              (Game|SpawnActorfromClass "/Game/GameBP/Blueprints/Actor/Bullet/ProjectileBP.ProjectileBP_C" (Math|Transform|MakeTransform _returnvalue (Math|Rotator|FindLookatRotation _returnvalue (Math|Vector|SelectVector (.ImpactPoint (Collision|BreakHitResult _outhit)) (.TraceEnd (Collision|BreakHitResult _outhit)) _returnvalue_3))) "Undefined" 0 0))))))))

(event Custom|StopFire
  (bind _aibasereference (Variables|Default|GetAIBaseReference))
  (bind _aibasereference_2 (Variables|Default|GetAIBaseReference))
  (bind _weapon (Variables|/Game/GameBP/Blueprints/AI/AskerYZ_BP.AskerYZ_BP_C|GetWeapon _aibasereference))
  (bind _weapon_2 (Variables|/Game/GameBP/Blueprints/AI/AskerYZ_BP.AskerYZ_BP_C|GetWeapon _aibasereference_2))
  (bind _skeletalmesh (Variables|/Game/GameBP/Blueprints/Actor/Weapon/WeaponBP.WeaponBP_C|GetSkeletalMesh _weapon))
  (bind _skeletalmesh_2 (Variables|/Game/GameBP/Blueprints/Actor/Weapon/WeaponBP.WeaponBP_C|GetSkeletalMesh _weapon_2))
  (bind _returnvalue (Transformation|GetSocketLocation _skeletalmesh "Muzzle"))
  (bind _returnvalue_2 (Transformation|GetSocketLocation _skeletalmesh_2 "Muzzle"))
  (Utilities|FlowControl|Gate true) ; enters at Close
)

(event EventBeginPlay
  (bind _asasker_yz_bp (Utilities|Casting|CastToAskerYZ_BP (Pawn|GetControlledPawn)))
  (Variables|Default|SetAIBaseReference _asasker_yz_bp)
  (Variables|Default|SetWayPoints (Variables|/Game/GameBP/Blueprints/AI/AskerYZ_BP.AskerYZ_BP_C|GetWayPoint _asasker_yz_bp))
  (bind _returnvalue (Utilities|Time|SetTimerbyFunctionName 0 "CheckEnemy" 0.3 true))
  (Variables|Default|SetCleanTimer _returnvalue)
  (AI|AIMoveTo _asasker_yz_bp "0, 0, 0" (Utilities|Array|Get(acopy) (Variables|Default|GetWayPoints) (Variables|Default|GetCurrentWayPoint)) 5.0 false
    (:OnSuccess
      (Utilities|FlowControl|Delay 3.0)
      (CallFunction|Patrolling))))

(fn ConstructionScript)