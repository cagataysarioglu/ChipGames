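; AI soldier enemy that spots TeomanPlayer, carries a weapon and can drop a health pack on death.
; Pawn sensing or non-head damage sets EnemyFound, which AlertSense overlaps spread between soldiers, with a pause on encountering dead ones.
; A forward trace updates Active for combat, while a FlipFlop moves the weapon between back and hand sockets.
; Headshots kill instantly; death ragdolls the body, removes the weapon, then spawns loot after a delay.
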(event OnSeePawn(PawnSensing)
  (params (Pawn :type Pawn%20Object%20Reference))
  (Utilities|Casting|CastToTeomanPlayer Pawn)
  (Variables|Default|SetEnemyFound true))

(event OnComponentBeginOverlap(AlertSense)
  (params (OverlappedComponent :type Primitive%20Component%20Object%20Reference) (OtherActor :type Actor%20Object%20Reference) (OtherComp :type Primitive%20Component%20Object%20Reference) (OtherBodyIndex :type Integer) (bFromSweep :type Boolean) (SweepResult :type Hit%20Result%20Structure%20%28by%20ref%29))
  (if (not (Variables|Default|GetEnemyFound))
    (Utilities|ActiveSense OtherActor)))

(event OnComponentEndOverlap(AlertSense)
  (params (OverlappedComponent :type Primitive%20Component%20Object%20Reference) (OtherActor :type Actor%20Object%20Reference) (OtherComp :type Primitive%20Component%20Object%20Reference) (OtherBodyIndex :type Integer))
  (if (not (Variables|Default|GetEnemyFound))
    (Utilities|ActiveSense OtherActor)))

(event Custom|EquipUnequip
  (Utilities|FlowControl|FlipFlop
    (:A
      (Transformation|AttachComponentToComponent (Variables|Default|GetWeapon) (Variables|Character|GetMesh) "HandWeapon" "KeepRelative" "KeepRelative" "KeepRelative" true)
      (Variables|Default|SetEquipWeapon true))
    (:B
      (Transformation|AttachComponentToComponent (Variables|Default|GetWeapon) (Variables|Character|GetMesh) "BackWeapon" "KeepRelative" "KeepRelative" "KeepRelative" true)
      (Variables|Default|SetEquipWeapon false)
      (Variables|Default|SetEnemyFound false))))

(event Custom|SpawnDefaultWeapon
  (bind _returnvalue (Game|SpawnActorfromClass (Variables|Default|GetWeaponClass) (Transformation|GetWorldTransform (Variables|Default|GetSphere)) "AlwaysSpawn" 0 0))
  (bind _output_get (Variables|Default|SetWeapon _returnvalue))
  (Transformation|AttachComponentToComponent _output_get (Variables|Character|GetMesh) "BackWeapon" "KeepWorld" "KeepWorld" "KeepWorld" true)
  (Default|DestroySphere _output_get))

(event Custom|EnableCombat
  (Animation|PlayAnimMontage "/Game/Models/Animations/AskerBir/AskerBir_SilahKusanmaMontage.AskerBir_SilahKusanmaMontage" 1.0 "None"))

(event Custom|ScanEnemy
  (bind _visiondirectionarrow (Variables|Default|GetVisionDirectionArrow))
  (bind _returnvalue (Transformation|GetWorldLocation _visiondirectionarrow))
  (bind (_outhit _returnvalue_2) (Collision|LineTraceByChannel _returnvalue (+ _returnvalue (* (Math|Vector|GetForwardVector _visiondirectionarrow) 3e+03)) "TraceTypeQuery1" true (Utilities|Array|MakeArray self) "None"))
  (if _returnvalue_2
    (if (Utilities|DoesObjectImplementInterface (.HitActor (Collision|BreakHitResult _outhit)) "/Game/GameBP/Blueprints/AI/TakeDamage.TakeDamage_C")
      (Utilities|Casting|CastToTeomanPlayer (.HitActor (Collision|BreakHitResult _outhit)))
      (Variables|Default|SetActive true)
      (else
        (Variables|Default|SetActive false)))))

(event Custom|SpawnItem
  (switch Utilities|FlowControl|Switch|SwitchonItemEnumerator (Variables|Default|GetRandomItem)
    (:NewEnumerator1
      (Variables|Default|SetItemClass "/Game/GameBP/Blueprints/Actor/Health_Key/HealthPack.HealthPack_C")
      (bind _returnvalue (Game|SpawnActorfromClass (Variables|Default|GetItemClass) (Math|Transform|MakeTransform (.Location (Math|Transform|BreakTransform (Transformation|GetSocketTransform (Variables|Character|GetMesh) "Hips" "RTS_World")))) "Undefined" 0 0))
      (Physics|SetSimulatePhysics (Variables|/Game/GameBP/Blueprints/Actor/Health_Key/ItemBP.ItemBP_C|GetStaticMesh _returnvalue) true))))

(event EventBeginPlay
  (Variables|Default|SetCurrentHealth (Variables|Default|GetMaxHealth))
  (CallFunction|SpawnDefaultWeapon))

(event EventITakeDamage
  (params (BoneName :type Name :default "None") (Damage :type Float%20%28single-precision%29))
  (if (Utilities|Name|Equal(Name) BoneName "Head")
    (Variables|Default|SetCurrentHealth 0.0)
    ;[1 1 1] Kafadan vurulma sesi
    (Audio|PlaySoundatLocation 0 (Transformation|GetWorldLocation (Variables|Character|GetMesh)) "0, 0, 0" 1.0 1.0 0.0 0 0 0)
    (Utilities|FlowControl|DoOnce false :!label _label
      (:Completed
        (Variables|Default|SetIsDead true)
        ;[1 1 1] Ölme animasyonu
        (Animation|PlayAnimMontage 0 1.0 "None")
        (Class|SkeletalMeshComponent|SetAllBodiesSimulatePhysics (Variables|Character|GetMesh) true)
        (Collision|SetCollisionEnabled (Variables|Collision|GetCapsuleComponent) "NoCollision")
        (Components|DestroyComponent (Variables|Default|GetAlertSense))
        (Actor|DestroyActor (Variables|Default|GetWeapon))
        (Utilities|FlowControl|Delay 13.0)
        (CallFunction|SpawnItem)
        (Actor|DestroyActor)))
    (else
      (Variables|Default|SetEnemyFound true)
      (Variables|Default|SetCurrentHealth (- (Variables|Default|GetCurrentHealth) Damage))
      (if (<= (Variables|Default|GetCurrentHealth) 0.0)
        (goto _label)))))

(fn ConstructionScript)