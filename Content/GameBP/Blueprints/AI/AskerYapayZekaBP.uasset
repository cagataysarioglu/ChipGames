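; Enemy soldier AI character that carries a spawned weapon and can be killed by damage.
; On BeginPlay it fills health and spawns its weapon on the back socket.
; Headshots kill instantly with a sound; other hits subtract health and flag an enemy as found, with death triggering a montage, ragdoll and disabled capsule collision.
; EnableCombat plays the draw montage, while EquipUnequip toggles the weapon between hand and back sockets via FlipFlop.
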(event Custom|EquipUnequip
  (Utilities|FlowControl|FlipFlop
    (:A
      (Transformation|AttachComponentToComponent (Variables|Default|GetWeapon) (Variables|Character|GetMesh) "HandWeapon" "KeepRelative" "KeepRelative" "KeepRelative" true)
      (Variables|Default|SetEquipWeapon true))
    (:B
      (Transformation|AttachComponentToComponent (Variables|Default|GetWeapon) (Variables|Character|GetMesh) "BackWeapon" "KeepWorld" "KeepWorld" "KeepWorld" true)
      (Variables|Default|SetEquipWeapon false))))

(event Custom|SpawnDefaultWeapon
  (bind _returnvalue (Game|SpawnActorfromClass (Variables|Default|GetWeaponClass) (Transformation|GetWorldTransform (Variables|Default|GetSphere)) "AlwaysSpawn" 0 0))
  (bind _output_get (Variables|Default|SetWeapon _returnvalue))
  (Transformation|AttachComponentToComponent _output_get (Variables|Character|GetMesh) "BackWeapon" "KeepWorld" "KeepWorld" "KeepWorld" true)
  (Default|DestroySphere _output_get))

(event Custom|EnableCombat
  (Animation|PlayAnimMontage "/Game/Models/Animations/AskerBir/AskerBir_SilahKusanmaMontage.AskerBir_SilahKusanmaMontage" 1.0 "None"))

(event EventBeginPlay
  (Variables|Default|SetCurrentHealth (Variables|Default|GetMaxHealth))
  (CallFunction|SpawnDefaultWeapon))

(event EventITakeDamage
  (params (BoneName :type Name :default "None") (Damage :type Float%20%28single-precision%29))
  (if (Utilities|Name|Equal(Name) BoneName "Head")
    (Variables|Default|SetCurrentHealth 0.0)
    ;[1 1 1] Kafadan vurulma sesi
    (Audio|PlaySoundatLocation 0 (Transformation|GetWorldLocation (Variables|Character|GetMesh)) "0, 0, 0" 1.0 1.0 0.0 0 0 0)
    (else
      (Variables|Default|SetEnemyFound true)
      (Variables|Default|SetCurrentHealth (- (Variables|Default|GetCurrentHealth) Damage))))
  (if (<= (Variables|Default|GetCurrentHealth) 0.0)
    (Variables|Default|SetIsDead true)
    ;[1 1 1] Ölme animasyonu
    (Animation|PlayAnimMontage 0 1.0 "None")
    (Class|SkeletalMeshComponent|SetAllBodiesSimulatePhysics (Variables|Character|GetMesh) true)
    (Collision|SetCollisionEnabled (Variables|Collision|GetCapsuleComponent) "NoCollision")))

(fn ConstructionScript)