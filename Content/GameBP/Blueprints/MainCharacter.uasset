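; Player character Blueprint for a shooter, handling movement, sprint, crouch, aiming, shooting and armor-backed health.
; BeginPlay creates the HUD and crosshair, then attaches a spawned M4A1 to the hand socket.
; Fire loops on the weapon's fire-rate delay, aiming swaps cameras, and a timeline eases sprint speed.
; Tick regenerates armor and spreads the crosshair by velocity, while fixed-step TakeDamage functions spill armor overflow into health.
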(event EventBeginPlay
  ;[1 1 1] Oynanış arayüzü
  (bind _returnvalue (UserInterface|CreateWidget "/Game/UI/MainHUD.MainHUD_C"))
  (UserInterface|Viewport|AddtoViewport _returnvalue 0)
  (bind _returnvalue_2 (UserInterface|CreateWidget "/Game/GameBP/Blueprints/DynamicCrosshair.WBCrosshair_C"))
  (bind _output_get (Variables|Default|SetCrosshairRef _returnvalue_2))
  (UserInterface|Viewport|AddtoViewport _output_get 0)
  (bind _returnvalue_3 (Game|SpawnActorfromClass "/Game/GameBP/Blueprints/Actor/Weapon/M4A1.M4A1_C" (Math|Transform|MakeTransform "0, 0, 0") "Undefined" 0 0))
  (bind _output_get_2 (Variables|Default|SetEquippedWeapon _returnvalue_3))
  (Transformation|AttachComponentToComponent _output_get_2 (Variables|Character|GetMesh) "HandWeapon" "SnapToTarget" "SnapToTarget" "SnapToTarget" true))

(event EventTick
  (params (DeltaSeconds :type Float%20%28single-precision%29))
  ;[1 1 1] Ekran göstergeleri
  (Utilities|FlowControl|Sequence
    (:then_0
      (Utilities|FlowControl|Delay 1.0)
      (if (< (Variables|Default|GetArmor) 1.0)
        (Variables|Default|SetArmor (+ (Variables|Default|GetArmor) 0.01))))
    (:then_1
      (Variables|/Game/GameBP/Blueprints/DynamicCrosshair.WBCrosshair_C|Setcrosshair_spread (Variables|Default|GetCrosshairRef) (Math|Float|MapRangeClamped (Math|Vector|VectorLength (Transformation|GetVelocity)) 0.0 4.5e+02 5.0 8e+01)))))

(event Input|ActionEvents|InputActionShoot
  (params (Key :type Key%20Structure :default "None"))
  (bind _equippedweapon (Variables|Default|GetEquippedWeapon))
  ;[1 1 1] Ateş etme
  (:Pressed
    (if (not (or (Variables|Default|GetIsSprinted) (Variables|Default|GetIsReloding))) :!label _label
      (if (> (Variables|/Game/GameBP/Blueprints/Actor/Weapon/Weapon.Weapon_C|GetAmmo (Variables|Default|GetEquippedWeapon)) 0)
        (Variables|Default|SetIsFiring true)
        (Default|Fire _equippedweapon)
        (Utilities|FlowControl|Delay (Variables|/Game/GameBP/Blueprints/Actor/Weapon/Weapon.Weapon_C|GetFireRate _equippedweapon))
        (if (Variables|Default|GetIsFiring)
          (goto _label)))))
  (:Released
    (Variables|Default|SetIsFiring false)))

(event Input|ActionEvents|InputActionSprint
  (params (Key :type Key%20Structure :default "None"))
  ;[1 1 1] Yumuşak yavaşlama ve hızlanma
  (:Pressed
    (bind _speed (Timeline|SpeedSmooth Play)
      (:Update
        (Variables|/Script/Engine.CharacterMovementComponent|SetMaxWalkSpeed (Variables|Character|GetCharacterMovement) _speed))))
  (:Released
    (Timeline|SpeedSmooth Reverse)))

(event Input|ActionEvents|InputActionCrouch
  (params (Key :type Key%20Structure :default "None"))
  (bind _charactermovement (Variables|Character|GetCharacterMovement))
  ;[1 1 1] Çömelme
  (:Pressed
    (if (Variables|Default|GetIsSprinted)
      (Variables|Default|SetIsSprinted false))
    (Variables|Default|SetIsCrouched true)
    (Variables|/Script/Engine.CharacterMovementComponent|SetMaxWalkSpeed _charactermovement 3e+02))
  (:Released
    (Variables|Default|SetIsCrouched false)
    (Variables|/Script/Engine.CharacterMovementComponent|SetMaxWalkSpeed _charactermovement 6e+02)))

(event Input|ActionEvents|InputActionSprint
  (params (Key :type Key%20Structure :default "None"))
  (bind _charactermovement (Variables|Character|GetCharacterMovement))
  ;[1 1 1] Depar atma
  (:Pressed
    (if (Variables|Default|GetIsCrouched)
      (Variables|Default|SetIsCrouched false))
    (Variables|Default|SetIsSprinted true)
    (Variables|/Script/Engine.CharacterMovementComponent|SetMaxWalkSpeed _charactermovement 1e+03))
  (:Released
    (Variables|Default|SetIsSprinted false)
    (Variables|/Script/Engine.CharacterMovementComponent|SetMaxWalkSpeed _charactermovement 6e+02)))

(event Input|ActionEvents|InputActionAimDownSights
  (params (Key :type Key%20Structure :default "None"))
  (bind _charactermovement (Variables|Character|GetCharacterMovement))
  ;[1 1 1] Nişan alma
  (:Pressed
    (Components|Activation|Deactivate (Variables|MyCharacter|GetFollowCamera))
    (Components|Activation|Activate (Variables|Default|GetADSCamera) false)
    (Variables|/Script/Engine.CharacterMovementComponent|SetMaxWalkSpeed _charactermovement 3e+02)
    (Variables|Default|SetAiming true))
  (:Released
    (Components|Activation|Deactivate (Variables|Default|GetADSCamera))
    (Components|Activation|Activate (Variables|MyCharacter|GetFollowCamera) false)
    (Variables|/Script/Engine.CharacterMovementComponent|SetMaxWalkSpeed _charactermovement 6e+02)
    (Variables|Default|SetAiming false)))

(event Input|ActionEvents|InputActionReload
  (params (Key :type Key%20Structure :default "None"))
  ;[1 1 1] Şarjör yükleme
  (:Pressed
    (bind (_outputone _outputtwo) (Default|Reload (Variables|Default|GetEquippedWeapon)))
    (if (or _outputone _outputtwo)
      (Utilities|FlowControl|Delay 3.3)
      (Variables|Default|SetIsReloding false))))

(event Input|ActionEvents|InputActionJump
  (params (Key :type Key%20Structure :default "None"))
  ;[1 1 1] Zıplama
  (:Pressed
    (Character|Jump))
  (:Released
    (Character|StopJumping)))

(event Input|AxisEvents|InputAxisLookUp
  (params (AxisValue :type Float%20%28single-precision%29))
  ;[1 1 1] Fare girdisi
  (Pawn|Input|AddControllerPitchInput AxisValue))

(event Input|AxisEvents|InputAxisTurnRate
  (params (AxisValue :type Float%20%28single-precision%29))
  ;[1 1 1] Gamepad girdisi
  (Pawn|Input|AddControllerYawInput (* AxisValue (Variables|Default|GetBaseTurnRate) (Utilities|Time|GetWorldDeltaSeconds))))

(event Input|AxisEvents|InputAxisTurn
  (params (AxisValue :type Float%20%28single-precision%29))
  ;[1 1 1] Fare girdisi
  (Pawn|Input|AddControllerYawInput AxisValue))

(event Input|AxisEvents|InputAxisLookUpRate
  (params (AxisValue :type Float%20%28single-precision%29))
  ;[1 1 1] Gamepad girdisi
  (Pawn|Input|AddControllerPitchInput (* AxisValue (Variables|Default|GetBaseLookUpRate) (Utilities|Time|GetWorldDeltaSeconds))))

(event Input|AxisEvents|InputAxisMoveForward
  (params (AxisValue :type Float%20%28single-precision%29))
  ;[1 1 1] Hareket girdisi
  (Pawn|Input|AddMovementInput (Math|Vector|GetForwardVector (Math|Rotator|MakeRotator 0.0 0.0 (.Yaw (Math|Rotator|BreakRotator (Pawn|GetControlRotation :!class /Script/Engine.Pawn))))) AxisValue false))

(event Input|AxisEvents|InputAxisMoveRight
  (params (AxisValue :type Float%20%28single-precision%29))
  ;[1 1 1] Hareket girdisi
  (Pawn|Input|AddMovementInput (Math|Vector|GetRightVector (Math|Rotator|MakeRotator 0.0 0.0 (.Yaw (Math|Rotator|BreakRotator (Pawn|GetControlRotation :!class /Script/Engine.Pawn))))) AxisValue false))

(event Input|TouchEvents|InputTouch
  (params (Location :type Vector) (FingerIndex :type ETouchIndex%20Enum))
  ;[1 1 1] Dokunuş girdisi
  (:Pressed
    (Character|Jump))
  (:Released
    (Character|StopJumping)))

(fn ConstructionScript)

(fn TakeDamage5
  (bind _output_get (Variables|Default|SetArmor (- (Variables|Default|GetArmor) 0.05)))
  (if (< _output_get 0.0)
    (Variables|Default|SetHealth (+ (Variables|Default|GetArmor) (Variables|Default|GetHealth)))
    (Variables|Default|SetArmor 0.0))
  (bind _returnvalue (UserInterface|CreateWidget "/Game/UI/DamageVignette.DamageVignette_C" (Game|GetPlayerController 0)))
  (UserInterface|Viewport|AddtoViewport _returnvalue 0))

(fn TakeDamage10
  (bind _output_get (Variables|Default|SetArmor (- (Variables|Default|GetArmor) 0.1)))
  (if (< _output_get 0.0)
    (Variables|Default|SetHealth (+ (Variables|Default|GetArmor) (Variables|Default|GetHealth)))
    (Variables|Default|SetArmor 0.0)))

(fn TakeDamage15
  (bind _output_get (Variables|Default|SetArmor (- (Variables|Default|GetArmor) 0.15)))
  (if (< _output_get 0.0)
    (Variables|Default|SetHealth (+ (Variables|Default|GetArmor) (Variables|Default|GetHealth)))
    (Variables|Default|SetArmor 0.0)))

(fn TakeDamage20
  (bind _output_get (Variables|Default|SetArmor (- (Variables|Default|GetArmor) 0.2)))
  (if (< _output_get 0.0)
    (Variables|Default|SetHealth (+ (Variables|Default|GetArmor) (Variables|Default|GetHealth)))
    (Variables|Default|SetArmor 0.0)))