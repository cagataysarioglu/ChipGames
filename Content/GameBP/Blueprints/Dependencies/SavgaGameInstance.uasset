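; Game instance that opens the game's menu screens and tracks level unlock progress.
; One event per menu (main, map, load, settings, credits, quit) creates its widget, adds it to the viewport and switches to UI-only input with a visible cursor.
; The main menu event also plays the Closing_In sound through a DoOnce.
; UnlockLevel increments a counter and sets the matching flag for Level2 through Level7.
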(event Custom|ShowMainMenu
  (bind _returnvalue (Game|GetPlayerController 0))
  (bind _returnvalue_2 (UserInterface|CreateWidget "/Game/UI/Menu/MainMenuWBP.MainMenuWBP_C" _returnvalue))
  (UserInterface|Viewport|AddtoViewport _returnvalue_2 0)
  (Input|SetInputModeUIOnly _returnvalue _returnvalue_2 "DoNotLock")
  (Variables|/Script/Engine.PlayerController|SetbShowMouseCursor _returnvalue true)
  (Utilities|FlowControl|DoOnce false
    (:Completed
      (Audio|PlaySound2D "/Game/Sounds/Closing_In.Closing_In" 1.0 1.0 0.0 0 0))))

(event Custom|ShowMapMenu
  (bind _returnvalue (Game|GetPlayerController 0))
  (bind _returnvalue_2 (UserInterface|CreateWidget "/Game/UI/Menu/MapMenuWBP.MapMenuWBP_C" _returnvalue))
  (UserInterface|Viewport|AddtoViewport _returnvalue_2 0)
  (Input|SetInputModeUIOnly _returnvalue _returnvalue_2 "DoNotLock")
  (Variables|/Script/Engine.PlayerController|SetbShowMouseCursor _returnvalue true))

(event Custom|ShowSettingsMenu
  (bind _returnvalue (Game|GetPlayerController 0))
  (bind _returnvalue_2 (UserInterface|CreateWidget "/Game/UI/Menu/SettingsMenuWBP.SettingsMenuWBP_C" _returnvalue))
  (UserInterface|Viewport|AddtoViewport _returnvalue_2 0)
  (Input|SetInputModeUIOnly _returnvalue _returnvalue_2 "DoNotLock")
  (Variables|/Script/Engine.PlayerController|SetbShowMouseCursor _returnvalue true))

(event Custom|ShowQuitMenu
  (bind _returnvalue (Game|GetPlayerController 0))
  (bind _returnvalue_2 (UserInterface|CreateWidget "/Game/UI/Menu/QuitMenuWBP.QuitMenuWBP_C" _returnvalue))
  (UserInterface|Viewport|AddtoViewport _returnvalue_2 0)
  (Input|SetInputModeUIOnly _returnvalue _returnvalue_2 "DoNotLock")
  (Variables|/Script/Engine.PlayerController|SetbShowMouseCursor _returnvalue true))

(event Custom|ShowCredits
  (bind _returnvalue (Game|GetPlayerController 0))
  (bind _returnvalue_2 (UserInterface|CreateWidget "/Game/UI/Menu/CreditsMenuWBP.CreditsMenuWBP_C" _returnvalue))
  (UserInterface|Viewport|AddtoViewport _returnvalue_2 0)
  (Input|SetInputModeUIOnly _returnvalue _returnvalue_2 "DoNotLock")
  (Variables|/Script/Engine.PlayerController|SetbShowMouseCursor _returnvalue true))

(event Custom|ShowLoadMenu
  (bind _returnvalue (Game|GetPlayerController 0))
  (bind _returnvalue_2 (UserInterface|CreateWidget "/Game/UI/Menu/LoadMenuWBP.LoadMenuWBP_C" _returnvalue))
  (UserInterface|Viewport|AddtoViewport _returnvalue_2 0)
  (Input|SetInputModeUIOnly _returnvalue _returnvalue_2 "DoNotLock")
  (Variables|/Script/Engine.PlayerController|SetbShowMouseCursor _returnvalue true))

(fn UnlockLevel
  (bind _result (Math|Integer|IncrementInt (Variables|Default|GetLevelUnlock))
    (:%20%20
      (Variables|Default|SetLevelUnlock _result)
      (if (== (Variables|Default|GetLevelUnlock) 1)
        (Variables|Default|SetLevel_2 true)
        (elif (== (Variables|Default|GetLevelUnlock) 2)
          (Variables|Default|SetLevel_3 true)
          (elif (== (Variables|Default|GetLevelUnlock) 3)
            (Variables|Default|SetLevel_4 true)
            (elif (== (Variables|Default|GetLevelUnlock) 4)
              (Variables|Default|SetLevel_5 true)
              (elif (== (Variables|Default|GetLevelUnlock) 5)
                (Variables|Default|SetLevel_6 true)
                (elif (== (Variables|Default|GetLevelUnlock) 6)
                  (Variables|Default|SetLevel_7 true))))))))))